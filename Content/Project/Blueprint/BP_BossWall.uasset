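; BP_BossWall is a wall actor, named for a boss encounter, that lowers when its StartLoweringWall event is called.
; It caches its location on BeginPlay, and a timeline moves it downward from that point without sweep.
; When the timeline finishes, the cached start location is reset to zero.
; A second timeline for upward movement exists but is never triggered.
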(event `self.ReceiveBeginPlay`
  (set `self.StartLocation` (`self.K2_GetActorLocation`)))

(event `self.StartLoweringWall`
  (bind (_direction _newtrack_0) (`Timeline|Timeline`)
    (:`Update`
      (`self.K2_SetActorLocation` (+ (`KismetMathLibrary.MakeVector` 0.0 0.0 (* _newtrack_0 -100.0)) (`self.StartLocation`))))
    (:`Finished`
      (set `self.StartLocation` (0.0 0.0 0.0)))))

(fn `UserConstructionScript`)